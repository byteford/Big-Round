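; Platform actor that vanishes from under the player, named as a falling platform though it only disappears in place.
; When an OP_BP_Character begins overlapping the Box trigger, a 1.5-second delay precedes hiding the Cube and disabling its collision.
; When any overlap with the Box ends, a 1-second delay precedes restoring the Cube's visibility and collision, with no class check.
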(event OnComponentBeginOverlap(Box)
  (params (OtherActor :type Actor%20Object%20Reference) (OtherComp :type Primitive%20Component%20Object%20Reference) (OtherBodyIndex :type Integer) (bFromSweep :type Boolean) (SweepResult :type Hit%20Result%20Structure%20%28by%20ref%29))
  (bind _cube (Variables|Default|GetCube))
  (if (== (Utilities|GetClass OtherActor) "/Game/Blueprints/OP_BP_Character.OP_BP_Character_C")
    (Utilities|FlowControl|Delay 1.5)
    (Collision|SetCollisionEnabled _cube "NoCollision")
    (Rendering|SetVisibility _cube false false)))

(event OnComponentEndOverlap(Box)
  (params (OtherActor :type Actor%20Object%20Reference) (OtherComp :type Primitive%20Component%20Object%20Reference) (OtherBodyIndex :type Integer))
  (bind _cube (Variables|Default|GetCube))
  (Utilities|FlowControl|Delay 1.0)
  (Collision|SetCollisionEnabled _cube "QueryAndPhysics")
  (Rendering|SetVisibility _cube true false))

(event EventBeginPlay)

(event EventActorBeginOverlap
  (params (OtherActor :type Actor%20Object%20Reference)))

(event EventTick
  (params (DeltaSeconds :type Float%20%28single-precision%29)))

(event Collision|EventActorEndOverlap
  (params (OtherActor :type Actor%20Object%20Reference)))

(fn ConstructionScript)