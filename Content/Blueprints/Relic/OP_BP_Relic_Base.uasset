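; Base relic pickup actor that hands the relic to an OP_BP_Character.
; Sphere overlap sets the character's relic flag, triggers its teleport relic event, state change and achievement, then destroys the actor.
; Unless placed at spawn, a JustSpawned flag blocks immediate re-pickup until a character leaves the sphere.
; Taking damage returns the relic flag to whoever spawned it and changes their state.
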(event OnComponentBeginOverlap(Sphere)
  (params (OtherActor :type Actor%20Object%20Reference) (OtherComp :type Primitive%20Component%20Object%20Reference) (OtherBodyIndex :type Integer) (bFromSweep :type Boolean) (SweepResult :type Hit%20Result%20Structure%20%28by%20ref%29))
  (if (== (Utilities|GetClass OtherActor) "/Game/Blueprints/OP_BP_Character.OP_BP_Character_C")
    (if (not (Variables|Default|GetJustSpawned)) ; Stops the player from picking it straight back up when placed
      (bind _asop_bp_character (Utilities|Casting|CastToOP_BP_Character OtherActor))
      (Variables|/Game/Blueprints/OP_BP_Character.OP_BP_Character_C|SetHasRelic _asop_bp_character true)
      (Default|TeleportRelicEvent _asop_bp_character)
      (Default|ChangeState _asop_bp_character true)
      (Default|Achievement _asop_bp_character 15)
      (Actor|DestroyActor))))

(event OnComponentEndOverlap(Sphere)
  (params (OtherActor :type Actor%20Object%20Reference) (OtherComp :type Primitive%20Component%20Object%20Reference) (OtherBodyIndex :type Integer))
  (if (== (Utilities|GetClass OtherActor) "/Game/Blueprints/OP_BP_Character.OP_BP_Character_C")
    (if (Variables|Default|GetJustSpawned)
      (Variables|Default|SetJustSpawned false))))

(event Game|Damage|EventAnyDamage
  (params (Damage :type Float%20%28single-precision%29) (DamageType :type Damage%20Type%20Object%20Reference) (InstigatedBy :type Controller%20Object%20Reference) (DamageCauser :type Actor%20Object%20Reference))
  (bind _whospawnedme (Variables|Default|GetWhoSpawnedMe))
  (Variables|/Game/Blueprints/OP_BP_Character.OP_BP_Character_C|SetHasRelic _whospawnedme true)
  (Default|ChangeState _whospawnedme true)
  (Variables|Default|SetbAutoDestroyWhenFinished true))

(event EventBeginPlay
  (if (Variables|Default|GetPlacedAtSpawn)
    (Variables|Default|SetJustSpawned false)
    (else
      (Variables|Default|SetJustSpawned true))))

(event EventActorBeginOverlap
  (params (OtherActor :type Actor%20Object%20Reference)))

(event Collision|EventActorEndOverlap
  (params (OtherActor :type Actor%20Object%20Reference)))

(fn ConstructionScript
  (|CallParentFunction))