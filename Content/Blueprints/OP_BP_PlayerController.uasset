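; Player controller that runs level flow: menu or in-game HUD, pause, win and lose screens, and next-level loading.
; On play it loads saved data, parses the level number from the map name and destroys an already-collected bonus relic.
; Win, death and relic events drive the HUD and save through GameInstance interface messages, unlocking achievements, some by cause of death.
; U and L are debug keys printing saved data.
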(event Custom|SetBonusRelic
  (params (LevelBonusRelic :type Boolean))
  ;[1 1 1] Set Bonus Relic
  (Class|OPIFInterface|ISetBonusRelic(Message) (Game|GetGameInstance) (Variables|Default|GetLevelNumber) (Utilities|Struct|MakeOP_Struct_Level false LevelBonusRelic))
  (Default|SetBonusRelicHUD (Variables|Default|GetHudRef)))

(event Custom|LoseTheLevel
  (params (Type :type OP_EN_DeathBox%20Enum) (NewParam :type Damage%20Type%20Object%20Reference))
  ;[1 1 1] Losing the Level
  (CallFunction|Achievement 23) ; Achievement: Dead Archaeologists Society
  (if (== NewParam "/Game/Blueprints/DamageType/Fire.Fire_C")
    (CallFunction|Achievement 25) ; Achievement: Conflagulations!
    (elif (== NewParam "/Game/Blueprints/DamageType/Poison.Poison_C")
      (CallFunction|Achievement 20) ; Achievement:Jungle Fever
      (elif (== NewParam "/Game/Blueprints/DamageType/Spikes.Spikes_C")
        (CallFunction|Achievement 21) ; Achievement: Spikeful
      )))
  (CallFunction|Achievement 31) ; Achievement: Do you need help?
  (Utilities|FlowControl|Delay 2.0)
  (CallFunction|Death))

(event Custom|WinTheLevel
  (params (LevelNumber :type Integer) (LevelCompleted :type Boolean) (LevelBonusRelic :type Boolean) (LevelTime :type Float%20%28single-precision%29) (LevelAchievement :type Integer))
  ;[1 1 1] Winning the Level
  (CallFunction|Achievement LevelAchievement) ; Level Achievement
  (Default|DrawWinLevelHUD (Variables|Default|GetHudRef) self)
  (Variables|Default|SetbShowMouseCursor true)
  (CallFunction|Save LevelNumber LevelCompleted LevelBonusRelic LevelTime))

(event Custom|TESTBONUSRELIC
  (bind _levels (Class|OPIFInterface|IGetLevels(Message) (Game|GetGameInstance)))
  (bind _returnvalue (Game|GetCurrentLevelName true))
  (if (Class|KismetStringLibrary|IsNumeric (.RightS (Utilities|String|Split _returnvalue "Level")))
    (bind _output_get (Variables|Default|SetLevelNumber (Math|Conversions|ToInteger(Byte) (.RightS (Utilities|String|Split _returnvalue "Level")))))
    (if (Math|Boolean|Equal(Boolean) (.LevelBonusRelic (Utilities|Struct|BreakOP_Struct_Level (Utilities|Array|Get(acopy) _levels _output_get))) true)
      (bind _outactors (Actor|GetAllActorsOfClass "/Game/Blueprints/Relic/OP_BP_Relic_Bonus.OP_BP_Relic_Bonus_C"))
      (if (not (== (Utilities|Array|Length _outactors) 0))
        (Actor|DestroyActor (Utilities|Array|Get(acopy) _outactors))))))

(event EventBeginPlay
  (CallFunction|GetHudRef)
  (bind _returnvalue (Game|GetCurrentLevelName true))
  (if (Utilities|Enum|Equal(Enum) _returnvalue "OP_LVL_MenuMap")
    (Default|DrawMainMenuHUD (Variables|Default|GetHudRef) self)
    (Class|OPIFInterface|ILoadOptions(Message) (Game|GetGameInstance))
    (else
      (Variables|Default|SetbShowMouseCursor false)
      (Default|DrawinGameHUD (Variables|Default|GetHudRef))
      (Class|OPIFInterface|ILoadGame(Message) (Game|GetGameInstance))
      (CallFunction|Achievement 28) ; Achievement: Into the Jungle
      ;[1 0.01989 0] Comment
      (bind _asop_bp_character (Utilities|Casting|CastToOP_BP_Character (Pawn|GetControlledPawn)))
      (Variables|Default|SetCharacterRef _asop_bp_character)
      (CallFunction|TESTBONUSRELIC))))

(event Input|ActionEvents|InputActionPauseMenu
  (params (Key :type Key%20Structure :default "AnyKey"))
  ;[1 1 1] Pause Menu
  (:Pressed
    (Default|DrawPauseMenuHUD (Variables|Default|GetHudRef) self)
    (Variables|Default|SetbShowMouseCursor true)))

(event Input|KeyboardEvents|K
  (params (Key :type Key%20Structure :default "AnyKey"))
  ;[1 1 1] Save/Load Game Test
)

(event Input|KeyboardEvents|L
  (params (Key :type Key%20Structure :default "AnyKey"))
  (bind _returnvalue (Game|GetGameInstance))
  ;[1 1 1] Save/Load Game Test
  (:Pressed
    (Class|OPIFInterface|ILoadGame(Message) _returnvalue)
    (bind _levels (Class|OPIFInterface|IGetLevels(Message) _returnvalue))
    (Development|PrintString (Utilities|String|ToString(Float) (.leveltime (Utilities|Array|Get(acopy) _levels 1))))))

(event Input|KeyboardEvents|U
  (params (Key :type Key%20Structure :default "AnyKey"))
  ;[1 1 1] Save/Load Game Test
  (:Pressed
    (bind _achievements (Class|OPIFInterface|IGetAchievements(Message) (Game|GetGameInstance)))
    (for _array_element _achievements
      (Development|PrintString (Utilities|String|BuildString(Integer) (Class|KismetStringLibrary|BuildStringBool "" (Utilities|String|Append (.AchievementName (Utilities|Struct|BreakOP_Struct_Achievement _array_element)) ": ") (.AchievementUnlocked (Utilities|Struct|BreakOP_Struct_Achievement _array_element)) " & Progress = ") (Utilities|String|BuildString(Integer) "" "" (.AchievementProgress (Utilities|Struct|BreakOP_Struct_Achievement _array_element)) "/") (.AchievementCompletedProgress (Utilities|Struct|BreakOP_Struct_Achievement _array_element)))))))

(fn ConstructionScript)

(fn Save
  (params (LevelNumber :type Integer) (LevelCompleted :type Boolean) (LevelBonusRelic :type Boolean) (LevelTime :type Float%20%28single-precision%29))
  (Class|OPIFInterface|ISaveGame(Message) (Game|GetGameInstance) LevelNumber LevelCompleted LevelBonusRelic LevelTime))

(fn LoadNextLevel
  (bind _returnvalue (UserInterface|CreateWidget "/Game/Blueprints/UMG/OP_UMG_LoadingSCreen.OP_UMG_LoadingScreen_C" 0 (Utilities|String|StringToName (Utilities|String|BuildString(Integer) "" "OP_LVL_Level" (+ (Variables|Default|GetLevelNumber) 1)))))
  (UserInterface|Viewport|AddtoViewport _returnvalue 0))

(fn Achievement
  (params (Achievement%20ID :type Integer))
  (bind _returnvalue (Game|GetGameInstance))
  (bind _asop_bp_game_instance (Utilities|Casting|CastToOP_BP_GameInstance _returnvalue))
  (bind (_outachievement _show_) (Default|AchievementFunction _asop_bp_game_instance Achievement%20ID))
  (if _show_
    (bind _asop_bp_hud (Utilities|Casting|CastToOP_BP_HUD (HUD|GetHUD)))
    (Default|CanDrawAchievementHUD _asop_bp_hud _outachievement)
    (Class|OPIFInterface|ISaveAchievements(Message) _returnvalue)))

(fn SetAchievementProgress
  (params (NewParam :type Integer) (OP_Struct_Achievement :type OP%20Struct%20Achievement%20Structure%20%28by%20ref%29))
  (bind _asop_bp_game_instance (Utilities|Casting|CastToOP_BP_GameInstance (Game|GetGameInstance)))
  (Default|SetAchievementProgress _asop_bp_game_instance NewParam OP_Struct_Achievement))

(fn Death
  (bind _asop_bp_hud (Utilities|Casting|CastToOP_BP_HUD (HUD|GetHUD)))
  (Default|DrawLoseLevelHUD _asop_bp_hud self)
  (Variables|Default|SetbShowMouseCursor true)
  (Class|OPIFInterface|ISaveGame(Message) (Game|GetGameInstance) 0 false false 0.0))

(fn RepossessPawn
  (Pawn|Possess (Variables|Default|GetCharacterRef)))

(fn GetHudRef
  (bind _asop_bp_hud (Utilities|Casting|CastToOP_BP_HUD (HUD|GetHUD)))
  (Variables|Default|SetHudRef _asop_bp_hud))

(fn NewFunction0)

(fn SavedTimeIsBetter
  (params (NewParam :type Float%20%28single-precision%29) (Index :type Integer))
  (bind _levels (Class|OPIFInterface|IGetLevels(Message) (Game|GetGameInstance)))
  (if (== (.LevelTime (Utilities|Struct|BreakOP_Struct_Level (Utilities|Array|Get(acopy) _levels Index))) 0.0)
    (if (< NewParam 999999999999.0)
      _
      (else
        (return 999999999999.0)))
    (elif (< NewParam (.LevelTime (Utilities|Struct|BreakOP_Struct_Level (Utilities|Array|Get(acopy) _levels Index))))
      _
      (else
        (return (.LevelParTime (Utilities|Struct|BreakOP_Struct_Level (Utilities|Array|Get(acopy) _levels Index)))))))
  (return NewParam))