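; Fish logic component that moves its owning actor along a looping list of MovePoints and can damage the player.
; Each tick it eases toward the current target with a swept, delta-time lerp and faces it, advancing when close.
; The RandomMovement branch only targets the world origin.
; CollideWithPlayer applies fish damage to the player character, though nothing here calls it.
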(event EventBeginPlay
  (Variables|Default|SetMove2 (Transformation|GetActorLocation (Utilities|Array|Get(acopy) (Variables|Default|GetMovePoints)))))

(event EventTick
  (params (DeltaSeconds :type Float%20%28single-precision%29))
  (bind _returnvalue (Components|GetOwner))
  (bind _returnvalue_2 (Transformation|GetActorLocation _returnvalue))
  (bind _move2 (CallFunction|WorkOutMove2))
  (Transformation|SetActorLocation _returnvalue (Math|Vector|Lerp(Vector) _returnvalue_2 _move2 DeltaSeconds) true false)
  (Transformation|SetActorRotation _returnvalue (Math|Rotator|FindLookatRotation _returnvalue_2 _move2)))

(fn CollidewithPlayer
  (params (Other :type Actor%20Object%20Reference))
  (bind _asop_bp_character (Utilities|Casting|CastToOP_BP_Character Other))
  (Game|Damage|ApplyDamage _asop_bp_character 1.0 0 0 "/Game/Blueprints/DamageType/Fish.Fish_C"))

(fn WorkOutMove2
  (if (< (Math|Vector|VectorLength (- (Transformation|GetActorLocation (Components|GetOwner)) (Variables|Default|GetMove2))) 1e+01)
    (if (Variables|Default|Getrandom%20Movement)
      (Variables|Default|SetMove2 "0, 0, 0")
      (else
        (bind _move (CallFunction|WorkOutNonRandomMove))
        (Variables|Default|SetMove2 _move)))
    (return (Variables|Default|GetMove2))
    (else
      (return (Variables|Default|GetMove2)))))

(fn WorkOutNonRandomMove
  (if (< (+ (Variables|Default|GetLastPoint) 1) (Utilities|Array|Length (Variables|Default|GetMovePoints)))
    (Variables|Default|SetLastPoint (+ (Variables|Default|GetLastPoint) 1))
    (else
      (Variables|Default|SetLastPoint 0)))
  (return (Transformation|GetActorLocation (Utilities|Array|Get(acopy) (Variables|Default|GetMovePoints) (Variables|Default|GetLastPoint)))))