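; Conveyor belt actor that carries any actor overlapping its Box toward the far end.
; Overlap events maintain a list of actors, which Tick lerps toward a Sphere marker using Speed as a per-frame alpha, without delta time or sweep.
; The construction script sizes the Box from BoxSize and places the Sphere at its +X edge.
; An alternative physics-velocity push along X is present but never runs.
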(event OnComponentBeginOverlap(Box)
  (params (OtherActor :type Actor%20Object%20Reference) (OtherComp :type Primitive%20Component%20Object%20Reference) (OtherBodyIndex :type Integer) (bFromSweep :type Boolean) (SweepResult :type Hit%20Result%20Structure%20%28by%20ref%29))
  (Utilities|Array|Add (Variables|Default|GetActorToMove) OtherActor))

(event OnComponentEndOverlap(Box)
  (params (OtherActor :type Actor%20Object%20Reference) (OtherComp :type Primitive%20Component%20Object%20Reference) (OtherBodyIndex :type Integer))
  (Utilities|Array|RemoveItem (Variables|Default|GetActorToMove) OtherActor))

(event EventTick
  (params (DeltaSeconds :type Float%20%28single-precision%29))
  (for _array_element (Variables|Default|GetActorToMove)
    (Transformation|SetActorLocation _array_element (Math|Vector|Lerp(Vector) (Transformation|GetActorLocation _array_element) (Transformation|GetWorldLocation (Variables|Default|GetSphere)) (Variables|Default|GetSpeed)) false false)))

(fn ConstructionScript
  (bind _box (Variables|Default|GetBox))
  (bind _boxsize (Variables|Default|GetBoxSize))
  (bind _relativelocation (Variables|/Script/Engine.SceneComponent|GetRelativeLocation _box))
  (bind (_x _y _z) (Math|Vector|BreakVector _relativelocation))
  (Components|Box|SetBoxExtent _box _boxsize true)
  (Transformation|SetRelativeLocation (Variables|Default|GetSphere) (Math|Vector|MakeVector (+ (.X (Math|Vector|BreakVector _boxsize)) _x) _y _z) false false))