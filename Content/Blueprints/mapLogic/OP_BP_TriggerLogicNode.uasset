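; OP_BP_TriggerLogicNode is a resizable box trigger for map logic.
; The construction script sets the box extent from Size.
; Box begin overlap passes the other actor to OnTriggerEnter on OPBPTriggerLogic, and end overlap calls OnTriggerExit without an actor.
; Older in-graph checks for OP_BP_Character and OP_BP_Relic_Base remain but are disconnected and never run.
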(event OnComponentBeginOverlap(Box)
  (params (OtherActor :type Actor%20Object%20Reference) (OtherComp :type Primitive%20Component%20Object%20Reference) (OtherBodyIndex :type Integer) (bFromSweep :type Boolean) (SweepResult :type Hit%20Result%20Structure%20%28by%20ref%29))
  (Default|OnTriggerEnter (Variables|Default|GetOP_BP_TriggerLogic) OtherActor))

(event OnComponentEndOverlap(Box)
  (params (OtherActor :type Actor%20Object%20Reference) (OtherComp :type Primitive%20Component%20Object%20Reference) (OtherBodyIndex :type Integer))
  (Default|OnTriggerExit (Variables|Default|GetOP_BP_TriggerLogic)))

(event EventBeginPlay)

(event EventActorBeginOverlap
  (params (OtherActor :type Actor%20Object%20Reference)))

(event EventTick
  (params (DeltaSeconds :type Float%20%28single-precision%29)))

(event EventTick
  (params (DeltaSeconds :type Float%20%28single-precision%29)))

(fn ConstructionScript
  (Components|Box|SetBoxExtent (Variables|Default|GetBox) (Variables|Default|GetSize) true))