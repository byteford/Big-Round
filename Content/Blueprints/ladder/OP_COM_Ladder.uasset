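; Ladder component that lets an OP_BP_Character climb up and down its owning actor.
; Each tick a box overlap checks the first pawn found; move-up input starts climbing, stopping movement and disabling gravity until the box no longer finds the character.
; Climb input advances a normalized height, seeded from the entry position, that lerps only the character's Z between bottom and top points with sweep.
; The game instance's debug flag draws the box and endpoints.
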(event EventBeginPlay)

(event EventTick
  (params (DeltaSeconds :type Float%20%28single-precision%29))
  (CallFunction|DebugStuff)
  (bind _onladder (CallFunction|IsOverlapLadder))
  (if _onladder
    (CallFunction|MoveonLadder DeltaSeconds)))

(fn IsOverlapLadder
  (bind (_outactors _returnvalue) (Class|KismetSystemLibrary|BoxOverlapActorsNEW (+ (Transformation|GetActorLocation (Components|GetOwner)) (Variables|Default|Getoffset)) (Variables|Default|Getsize) (Utilities|Array|MakeArray "ObjectTypeQuery3")))
  (if _returnvalue
    (bind _asop_bp_character (Utilities|Casting|CastToOP_BP_Character (Utilities|Array|Get(acopy) _outactors))
      (:then
        (if (!= (Variables|/Game/Blueprints/OP_BP_Character.OP_BP_Character_C|GetMoveUpAmount _asop_bp_character) 0.0)
          (if (Variables|Default|GetonLadder)
            _
            (else
              (CallFunction|StartonLadder _asop_bp_character)
              (Variables|Default|SetonLadder true)))
          (Variables|Default|SetLastPlayer _asop_bp_character)
          (Variables|/Script/Engine.CharacterMovementComponent|SetGravityScale (Variables|/Script/Engine.Character|GetCharacterMovement _asop_bp_character) 0.0)))
      (:CastFailed
        (if (Variables|Default|GetonLadder) :!label _label
          (Variables|/Script/Engine.CharacterMovementComponent|SetGravityScale (Variables|/Script/Engine.Character|GetCharacterMovement (Variables|Default|GetLastPlayer)) 1.0)
          (Variables|Default|SetonLadder false))))
    (else
      (goto _label)))
  (return (Variables|Default|GetonLadder)))

(fn MoveonLadder
  (params (DeltaTime :type Float%20%28single-precision%29))
  (bind _returnvalue (Components|GetOwner))
  (bind _lastplayer (Variables|Default|GetLastPlayer))
  (bind _returnvalue_2 (Transformation|GetActorLocation _returnvalue))
  (bind _returnvalue_3 (Transformation|GetActorLocation _lastplayer))
  (bind (_x _y) (Math|Vector|BreakVector _returnvalue_3))
  (bind _output_get (Variables|Default|SetamountTravled (Math|Float|Clamp(Float) (+ (* DeltaTime (Variables|/Game/Blueprints/OP_BP_Character.OP_BP_Character_C|GetMoveUpAmount _lastplayer) (Variables|Default|GetClimSpeed)) (Variables|Default|GetamountTravled)))))
  (Transformation|SetActorLocation _lastplayer (Math|Vector|Lerp(Vector) (Math|Vector|MakeVector _x _y (.Z (Math|Vector|BreakVector (+ _returnvalue_2 (Variables|Default|GetBottemOfLadder))))) (Math|Vector|MakeVector _x _y (.Z (Math|Vector|BreakVector (+ _returnvalue_2 (Variables|Default|GetTopOfLadder))))) _output_get) true false))

(fn StartonLadder
  (params (Player :type OP%20BP%20Character%20Object%20Reference))
  (bind _returnvalue (Transformation|GetActorLocation Player))
  (bind _returnvalue_2 (Components|GetOwner))
  (bind _bottemofladder (Variables|Default|GetBottemOfLadder))
  (bind _topofladder (Variables|Default|GetTopOfLadder))
  (bind _z (Math|Vector|BreakVector _returnvalue))
  (bind _returnvalue_3 (Transformation|GetActorLocation _returnvalue_2))
  (bind _z_2 (Math|Vector|BreakVector _topofladder))
  (bind _returnvalue_4 (+ _bottemofladder _returnvalue_3))
  (bind _returnvalue_5 (* _z_2 2.0))
  (bind _z_3 (Math|Vector|BreakVector _returnvalue_4))
  (bind _returnvalue_6 (- _z _z_3))
  (bind _returnvalue_7 (/ _returnvalue_6 _returnvalue_5))
  (Components|Movement|StopMovementImmediately (Variables|/Script/Engine.Character|GetCharacterMovement Player))
  (Development|PrintString (Utilities|String|BuildString(Float) "" "total:" _returnvalue_7))
  (Variables|Default|SetamountTravled (Math|Float|Clamp(Float) _returnvalue_7)))

(fn DebugStuff
  (bind _returnvalue (Components|GetOwner))
  (bind _returnvalue_2 (Transformation|GetActorLocation _returnvalue))
  (bind _asop_bp_game_instance (Utilities|Casting|CastToOP_BP_GameInstance (Game|GetGameInstance)))
  (bind _debug_ (Default|IsShowDebug _asop_bp_game_instance))
  (if _debug_
    (Rendering|Debug|DrawDebugBox :Center (+ _returnvalue_2 (Variables|Default|Getoffset)) :Extent (Variables|Default|Getsize))
    (Rendering|Debug|DrawDebugSphere (+ _returnvalue_2 (Variables|Default|GetTopOfLadder)) 1e+02 12 "(R=1.000000,G=1.000000,B=1.000000,A=1.000000)" 0.0)
    (Rendering|Debug|DrawDebugSphere (+ _returnvalue_2 (Variables|Default|GetBottemOfLadder)) 1e+02 12 "(R=1.000000,G=1.000000,B=1.000000,A=1.000000)" 0.0)))