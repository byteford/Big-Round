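; Movement manager component for OP_BP_Character that switches the owner's CharacterMovement settings between fat, thin and crouching presets.
; The fat and thin functions cast the owner and set walk and crouched speeds from MovementValues.
; The crouching function instead uses hardcoded values, also setting step height, walkable floor, friction and braking deceleration.
; The event graph has no active logic, so the presets rely on outside callers.
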(event EventBeginPlay)

(event EventTick
  (params (DeltaSeconds :type Float%20%28single-precision%29)))

(fn FatMovementValues
  (bind _movementvalues (Variables|Default|GetMovementValues))
  (bind (_thinmaxwalkspeed _thinmaxwalkspeedcrouched _fatmaxwalkspeed _fatmaxwalkspeedcrouched) (Utilities|Struct|BreakOP_Struct_Movement _movementvalues))
  (bind _asop_bp_character (Utilities|Casting|CastToOP_BP_Character (Components|GetOwner)))
  (Variables|/Script/Engine.CharacterMovementComponent|SetMaxWalkSpeed (Variables|/Script/Engine.Character|GetCharacterMovement _asop_bp_character) _fatmaxwalkspeed)
  (Variables|/Script/Engine.CharacterMovementComponent|SetMaxWalkSpeedCrouched (Variables|/Script/Engine.Character|GetCharacterMovement _asop_bp_character) _fatmaxwalkspeedcrouched))

(fn ThinMovementValues
  (bind _movementvalues (Variables|Default|GetMovementValues))
  (bind (_thinmaxwalkspeed _thinmaxwalkspeedcrouched) (Utilities|Struct|BreakOP_Struct_Movement _movementvalues))
  (bind _asop_bp_character (Utilities|Casting|CastToOP_BP_Character (Components|GetOwner)))
  (Variables|/Script/Engine.CharacterMovementComponent|SetMaxWalkSpeed (Variables|/Script/Engine.Character|GetCharacterMovement _asop_bp_character) _thinmaxwalkspeed)
  (Variables|/Script/Engine.CharacterMovementComponent|SetMaxWalkSpeedCrouched (Variables|/Script/Engine.Character|GetCharacterMovement _asop_bp_character) _thinmaxwalkspeedcrouched))

(fn CrouchingMovementValues
  (bind _asop_bp_character (Utilities|Casting|CastToOP_BP_Character (Components|GetOwner)))
  (Variables|/Script/Engine.CharacterMovementComponent|SetMaxStepHeight (Variables|/Script/Engine.Character|GetCharacterMovement _asop_bp_character) 45.0)
  (Pawn|Components|CharacterMovement|SetWalkableFloorAngle (Variables|/Script/Engine.Character|GetCharacterMovement _asop_bp_character) 44.765083)
  (Class|CharacterMovementComponent|SetWalkableFloorZ (Variables|/Script/Engine.Character|GetCharacterMovement _asop_bp_character) 0.71)
  (Variables|/Script/Engine.CharacterMovementComponent|SetGroundFriction (Variables|/Script/Engine.Character|GetCharacterMovement _asop_bp_character) 8.0)
  (Variables|/Script/Engine.CharacterMovementComponent|SetMaxWalkSpeed (Variables|/Script/Engine.Character|GetCharacterMovement _asop_bp_character) 6e+02)
  (Variables|/Script/Engine.CharacterMovementComponent|SetMaxWalkSpeedCrouched (Variables|/Script/Engine.Character|GetCharacterMovement _asop_bp_character) 3e+02)
  (Variables|/Script/Engine.CharacterMovementComponent|SetBrakingDecelerationWalking (Variables|/Script/Engine.Character|GetCharacterMovement _asop_bp_character) 2048.0))