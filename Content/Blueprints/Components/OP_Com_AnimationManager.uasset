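; Player animation manager component that picks the sprite's flipbook from movement and action flags.
; Each Tick runs state checks in sequence, so later ones override earlier ones; death has no reset.
; The state plus a player-size offset indexes one flat Flipbooks array covering every size.
; It also yaws the controller to face horizontal travel, snapping to the positive-X facing at zero X velocity.
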(event EventBeginPlay)

(event EventTick
  (params (DeltaSeconds :type Float%20%28single-precision%29))
  (CallFunction|IsRunning)
  (CallFunction|IsJumping)
  (CallFunction|IsGrappling)
  (CallFunction|IsTeleporting)
  (CallFunction|IsThrowingGrapple)
  (CallFunction|IsSwimming)
  (CallFunction|IsDead)
  (CallFunction|NextAnimfromEnum)
  (Sprite|SetFlipbook (Variables|Default|GetPlayerSprite) (Utilities|Array|Get(acopy) (Variables|Default|GetFlipbooks) (Variables|Default|GetNextAnimation)))
  (CallFunction|RunningDirection))

(fn IsRunning
  (if (> (Math|Vector|VectorLength (Variables|PlayerVars|GetPlayerVelocity)) 0.0)
    (if (Utilities|Enum|Equal(Enum) (Variables|PlayerVars|GetPlayerState) "NewEnumerator10")
      (Variables|PlayerVars|SetPlayerState "NewEnumerator0") ; throw grapple
    )
    (elif (Utilities|Enum|Equal(Enum) (Variables|PlayerVars|GetPlayerState) "NewEnumerator0")
      (Variables|PlayerVars|SetPlayerState "NewEnumerator10") ; walking
    )))

(fn Init
  (params (PlayerSprite :type Paper%20Flipbook%20Component%20Object%20Reference) (PlayerController :type Controller%20Object%20Reference))
  (Variables|Default|SetPlayerSprite PlayerSprite)
  (Variables|PlayerVars|SetPlayerController PlayerController)
  (bind _output_get (Variables|PlayerVars|SetPlayerState "NewEnumerator10"))
  (Sprite|SetFlipbook (Variables|Default|GetPlayerSprite) (Utilities|Array|Get(acopy) (Variables|Default|GetFlipbooks) (Math|Conversions|ToInteger(Byte) _output_get))))

(fn RunningDirection
  (bind _playercontroller (Variables|PlayerVars|GetPlayerController))
  (Math|Float|CompareFloat (.X (Math|Vector|BreakVector (Variables|PlayerVars|GetPlayerVelocity))) 0.0
    (:>
      (Pawn|SetControlRotation _playercontroller (Math|Rotator|MakeRotator 0.0 0.0 0.0) :!label _label))
    (:==
      (goto _label))
    (:<
      (Pawn|SetControlRotation _playercontroller (Math|Rotator|MakeRotator 0.0 0.0 1.8e+02)))))

(fn NextAnimfromEnum
  (Variables|Default|SetNextAnimation (+ (Math|Conversions|ToInteger(Byte) (Variables|PlayerVars|GetPlayerState)) (* (Math|Conversions|ToInteger(Byte) (Variables|PlayerVars|GetPlayerSize)) (|GetNumEnumEntries)))))

(fn IsJumping
  (if (Variables|PlayerVars|GetPlayerJumping)
    (Variables|PlayerVars|SetPlayerState "NewEnumerator9")
    (elif (Utilities|Enum|Equal(Enum) (Variables|PlayerVars|GetPlayerState) "NewEnumerator9")
      (Variables|PlayerVars|SetPlayerState "NewEnumerator10"))))

(fn IsGrappling
  (if (Variables|PlayerVars|GetPlayerGrappling)
    (Variables|PlayerVars|SetPlayerState "NewEnumerator2")
    (elif (Utilities|Enum|Equal(Enum) (Variables|PlayerVars|GetPlayerState) "NewEnumerator2")
      (Variables|PlayerVars|SetPlayerState "NewEnumerator10"))))

(fn IsTeleporting
  (if (Variables|PlayerVars|GetPlayerTeleporting)
    (Variables|PlayerVars|SetPlayerState "NewEnumerator3")
    (elif (Utilities|Enum|Equal(Enum) (Variables|PlayerVars|GetPlayerState) "NewEnumerator3")
      (Variables|PlayerVars|SetPlayerState "NewEnumerator10"))))

(fn IsThrowingGrapple
  (if (Variables|PlayerVars|GetPlayerThrowingGrapple)
    (Variables|PlayerVars|SetPlayerState "NewEnumerator1")
    (elif (Utilities|Enum|Equal(Enum) (Variables|PlayerVars|GetPlayerState) "NewEnumerator1")
      (Variables|PlayerVars|SetPlayerState "NewEnumerator10"))))

(fn IsDead
  (if (Variables|PlayerVars|GetPlayerDead)
    (Variables|PlayerVars|SetPlayerState "NewEnumerator13")))

(fn IsSwimming
  (if (Variables|PlayerVars|GetPlayerSwimming)
    (Variables|PlayerVars|SetPlayerState "NewEnumerator4")
    (elif (Utilities|Enum|Equal(Enum) (Variables|PlayerVars|GetPlayerState) "NewEnumerator4")
      (Variables|PlayerVars|SetPlayerState "NewEnumerator10"))))