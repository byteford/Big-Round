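; OP_Com_Grappable is an actor component that holds grapple data for its owning actor.
; On BeginPlay it caches the owner's first StaticMeshComponent as the mesh, with no check that one exists.
; Getters expose that mesh, the level needed to grapple and whether the object is moveable; the component contains no grapple logic itself.
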(event EventBeginPlay
  (Variables|Default|SetMesh (Utilities|Array|Get(acopy) (Actor|GetComponentsByClass (Components|GetOwner self) "/Script/Engine.StaticMeshComponent"))))

(event EventTick
  (params (DeltaSeconds :type Float%20%28single-precision%29)))

(fn GetLeveltoGrapple
  (return (Variables|Default|GetLevelNeededToGrapple)))

(fn GetMesh
  (return (Variables|Default|GetMesh)))

(fn GetMoveable
  (return (Variables|Default|GetMoveAble)))