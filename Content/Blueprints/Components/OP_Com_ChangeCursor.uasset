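; Actor component that switches the HUD crosshair to a highlighted texture while the cursor is over its owning actor.
; On BeginPlay it binds to the owner's begin and end cursor-over events.
; Each handler finds the first OP_BP_PlayerController, casts its HUD to OP_BP_HUD and sets CursorTexture to the highlight or normal crosshair.
; Both handlers also print a debug string, and Tick is unused.
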(event Custom|Show%20Interactive%20Cursor
  (Development|PrintString "Hello")
  (bind _outactors (Actor|GetAllActorsOfClass "/Game/Blueprints/OP_BP_PlayerController.OP_BP_PlayerController_C"))
  (bind _asop_bp_hud (Utilities|Casting|CastToOP_BP_HUD (HUD|GetHUD (Utilities|Array|Get(acopy) _outactors))))
  (Variables|/Game/Blueprints/GameClasses/OP_BP_HUD.OP_BP_HUD_C|SetCursorTexture _asop_bp_hud "/Game/Blueprints/GameClasses/OP_TX_CrosshairHighlight.OP_TX_CrosshairHighlight"))

(event Custom|Show%20Normal%20Cursor
  (Development|PrintString "BYE")
  (bind _outactors (Actor|GetAllActorsOfClass "/Game/Blueprints/OP_BP_PlayerController.OP_BP_PlayerController_C"))
  (bind _asop_bp_hud (Utilities|Casting|CastToOP_BP_HUD (HUD|GetHUD (Utilities|Array|Get(acopy) _outactors))))
  (Variables|/Game/Blueprints/GameClasses/OP_BP_HUD.OP_BP_HUD_C|SetCursorTexture _asop_bp_hud "/Game/Blueprints/GameClasses/OP_TX_Crosshair.OP_TX_Crosshair"))

(event EventBeginPlay
  (bind _returnvalue (Components|GetOwner))
  (EventDispatchers|BindEventtoOnBeginCursorOver _returnvalue (delegate Custom|Show%20Interactive%20Cursor))
  (EventDispatchers|BindEventtoOnEndCursorOver _returnvalue (delegate Custom|Show%20Normal%20Cursor)))

(event EventTick
  (params (DeltaSeconds :type Float%20%28single-precision%29)))