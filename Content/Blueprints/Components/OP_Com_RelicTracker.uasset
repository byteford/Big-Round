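; Actor component that spawns a RelicTracker pointer actor to show its owner the direction of the relic.
; Tracking latches on once TrackRelic is set or the owning OP_BP_Character has a relic.
; Each tick FindRelic takes the first OP_BP_Relic_Base in the world, hiding the tracker mesh if none exists.
; Otherwise the tracker sits offset from the owner along the owner-relic line, rotated to face the relic.
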(event EventBeginPlay
  (bind _returnvalue (Game|SpawnActorfromClass "/Game/RelicTracker.RelicTracker_C" (Math|Transform|MakeTransform "0, 0, 0") "AlwaysSpawn" (Components|GetOwner) 0))
  (Variables|Default|SetRelicTracker _returnvalue))

(event EventTick
  (params (DeltaSeconds :type Float%20%28single-precision%29))
  (bind _returnvalue (Components|GetOwner))
  (bind _relictracker (Variables|Default|GetRelicTracker))
  (bind _playeroffset (Variables|Default|GetPlayerOffset))
  (bind _returnvalue_2 (Transformation|GetActorLocation _returnvalue))
  (bind _staticmesh (Variables|/Game/RelicTracker.RelicTracker_C|GetStaticMesh _relictracker))
  (bind _returnvalue_3 (+ _playeroffset _returnvalue_2))
  (if (Variables|Default|GetTrackRelic)
    (bind (_relic _canfind) (CallFunction|FindRelic :!label _label))
    (if _canfind
      (Rendering|SetVisibility _staticmesh true false)
      (Variables|Default|SetRelic _relic)
      (bind _output_get (Variables|Default|SetVectorToRelic (Math|Vector|Normalize (- _returnvalue_3 (Transformation|GetActorLocation (Variables|Default|GetRelic))))))
      (Transformation|SetRelativeLocationAndRotation (Variables|/Game/RelicTracker.RelicTracker_C|GetDefaultSceneRoot (Variables|Default|GetRelicTracker)) (+ (Variables|Default|GetLocation%20Offset) (+ (* _output_get (Variables|Default|Getoffset)) _returnvalue_3)) (Math|Rotator|FindLookatRotation _returnvalue_3 (Transformation|GetActorLocation (Variables|Default|GetRelic))) true false)
      (else
        (Rendering|SetVisibility _staticmesh false false)))
    (else
      (bind _asop_bp_character (Utilities|Casting|CastToOP_BP_Character _returnvalue))
      (if (Variables|/Game/Blueprints/OP_BP_Character.OP_BP_Character_C|GetHasRelic _asop_bp_character)
        (Variables|Default|SetTrackRelic true)
        (goto _label)))))

(fn FindRelic
  (bind _outactors (Actor|GetAllActorsOfClass "/Game/Blueprints/Relic/OP_BP_Relic_Base.OP_BP_Relic_Base_C"))
  (if (== (Utilities|Array|Length _outactors) 0) ; This stops me getting out of bounds errors in the menu!
    (return 0 false)
    (else
      (return (Utilities|Array|Get(acopy) _outactors) (> (Utilities|Array|Length _outactors) 0)))))