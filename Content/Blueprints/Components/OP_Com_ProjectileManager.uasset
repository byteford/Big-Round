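; Player component that manages aiming and ability input, passing mouse clicks and releases to an injected list of abilities.
; Init stores the controller and character and initializes each ability with itself; left click drives ability 0, right click fires ability 1, and QPressed stops it.
; Each tick and click updates MousePosition as a normalized XZ-plane aim direction, from the gamepad right stick when nonzero, otherwise from the deprojected mouse relative to FarCamera.
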(event EventBeginPlay)

(event EventTick
  (params (DeltaSeconds :type Float%20%28single-precision%29))
  (CallFunction|FindMousePos))

(fn Init
  (params (PlayerControler :type Player%20Controller%20Object%20Reference) (PlayerChar :type OP%20BP%20Character%20Object%20Reference) (Abilityes :type Array%20of%20OP%20Com%20Ability%20Object%20References))
  (Variables|Default|SetPlayerControler PlayerControler)
  (Variables|Default|SetPlayerCharacter PlayerChar)
  (Variables|Default|SetAbilities Abilityes)
  (for _array_element (Variables|Default|GetAbilities)
    (Default|Init _array_element self)))

(fn LeftMouseClick
  (CallFunction|FindMousePos)
  (bind _newparam (CallFunction|FireAbility))
  (return _newparam))

(fn FindMousePos
  (bind _playercontroler (Variables|Default|GetPlayerControler))
  (bind _playercharacter (Variables|Default|GetPlayerCharacter))
  (bind _gamepadrightvect (Variables|Default|GetGamePadRightVect))
  (bind _returnvalue (Math|Vector|NotEqual(Vector) _gamepadrightvect "0, 0, 0" 0.0))
  (bind (_x _y) (Math|Vector|BreakVector _gamepadrightvect))
  (bind _worldlocation (Game|Player|ConvertMouseLocationToWorldSpace _playercontroler))
  (bind _farcamera (Variables|/Game/Blueprints/OP_BP_Character.OP_BP_Character_C|GetFarCamera _playercharacter))
  (bind _returnvalue_2 (Transformation|GetWorldLocation _farcamera))
  (bind _returnvalue_3 (- _worldlocation _returnvalue_2))
  (bind (_x_2 _y_2 _z) (Math|Vector|BreakVector _returnvalue_3))
  (Variables|Default|SetUsingcont _returnvalue)
  (if _returnvalue
    (Variables|Default|Setmouse%20Position (Math|Vector|Normalize (Math|Vector|MakeVector _x 0.0 (* _y -1.0))))
    (else
      (Variables|Default|Setmouse%20Position (Math|Vector|Normalize (Math|Vector|MakeVector _x_2 0.0 _z))))))

(fn LeftMouseRelease
  (CallFunction|ReleaseAbilty))

(fn FireAbility
  (params (AbiltyNumber :type Integer))
  (bind _newparam (Default|FireAbility (Utilities|Array|Get(acopy) (Variables|Default|GetAbilities) AbiltyNumber)))
  (return _newparam))

(fn ReleaseAbilty
  (params (AbiltyNumber :type Integer))
  (Default|StopAbillity (Utilities|Array|Get(acopy) (Variables|Default|GetAbilities) AbiltyNumber)))

(fn RightMouseClick
  (CallFunction|FindMousePos)
  (bind _newparam (CallFunction|FireAbility 1))
  (return _newparam))

(fn QPressed
  (CallFunction|ReleaseAbilty 1))

(fn SetGamePadRightVectX
  (params (X :type Float%20%28single-precision%29))
  (Variables|Default|SetGamePadRightVect (Math|Vector|MakeVector X (.Y (Math|Vector|BreakVector (Variables|Default|GetGamePadRightVect))) (.Z (Math|Vector|BreakVector (Variables|Default|GetGamePadRightVect))))))

(fn SetGamePadRightVectY
  (params (Y :type Float%20%28single-precision%29))
  (Variables|Default|SetGamePadRightVect (Math|Vector|MakeVector (.X (Math|Vector|BreakVector (Variables|Default|GetGamePadRightVect))) Y (.Z (Math|Vector|BreakVector (Variables|Default|GetGamePadRightVect))))))