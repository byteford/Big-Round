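; Camera manager component that keeps a registry of cameras and switches which one is active.
; Cameras and names live in parallel arrays, registered with a given or object name and retrieved by index or name.
; ChangeCam deactivates every camera, activates the target and stores its index as current, while SwapCam toggles between two.
; ChangeCamWithName is unfinished: it ignores the name and passes no camera to ChangeCam.
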(event EventBeginPlay)

(event EventTick
  (params (DeltaSeconds :type Float%20%28single-precision%29)))

(fn AddCamerawithName
  (params (camera :type Camera%20Component%20Object%20Reference) (name :type String))
  (Utilities|Array|Add (Variables|Default|GetCameras) camera)
  (Utilities|Array|Add (Variables|Default|GetCameraNames) name)
  (return self))

(fn AddCamera
  (params (Camera :type Camera%20Component%20Object%20Reference))
  (bind _camman (CallFunction|AddCamerawithName Camera (Utilities|GetObjectName Camera)))
  (return _camman))

(fn GetCamera
  (params (number :type Integer))
  (return (Utilities|Array|Get(acopy) (Variables|Default|GetCameras) number)))

(fn GetCamerawithName
  (params (name :type String))
  (bind _camera (CallFunction|GetCamera (Utilities|Array|FindItem (Variables|Default|GetCameraNames) name)))
  (return _camera))

(fn ChangeCam
  (params (camera :type Camera%20Component%20Object%20Reference))
  (bind _number (CallFunction|FindCam camera))
  (CallFunction|UnActiveAll)
  (CallFunction|SetCamActive camera _number))

(fn UnActiveAll
  (for _array_element (Variables|Default|GetCameras)
    (Components|Activation|SetActive _array_element false false)))

(fn SetCamActive
  (params (Camera :type Camera%20Component%20Object%20Reference) (numbe :type Integer))
  (Components|Activation|SetActive Camera true false)
  (Variables|Default|SetcurrentCam numbe))

(fn ChangeCamwithName
  (params (name :type String))
  (CallFunction|ChangeCam))

(fn GetCurrentCam
  (bind _camera (CallFunction|GetCamera (Variables|Default|GetcurrentCam)))
  (return _camera))

(fn IsCamActive
  (params (camera :type Camera%20Component%20Object%20Reference))
  (return (Components|Activation|IsActive camera) self))

(fn FindCam
  (params (camera :type Camera%20Component%20Object%20Reference))
  (return (Utilities|Array|FindItem (Variables|Default|GetCameras) camera)))

(fn SwapCam
  (params (Cam1 :type Camera%20Component%20Object%20Reference) (Cam2 :type Camera%20Component%20Object%20Reference))
  (bind _isactive (CallFunction|IsCamActive Cam1))
  (if _isactive
    (CallFunction|ChangeCam Cam2)
    (else
      (CallFunction|ChangeCam Cam1))))