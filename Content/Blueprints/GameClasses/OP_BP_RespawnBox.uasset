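; OP_BP_RespawnBox is a trigger volume that applies a fixed amount of damage to any actor that begins overlapping it.
; The construction script sizes its box from a Length variable, with fixed width and height.
; Disconnected graph logic, which never runs, would make the player lose the level, return relics to their spawners, or destroy the overlapping actor.
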(event EventBeginPlay)

(event EventActorBeginOverlap
  (params (OtherActor :type Actor%20Object%20Reference))
  (Game|Damage|ApplyDamage OtherActor 1.0 0 0 (Variables|Default|GetDamageType)))

(event EventTick
  (params (DeltaSeconds :type Float%20%28single-precision%29)))

(fn ConstructionScript
  (Components|Box|SetBoxExtent (Variables|Default|GetBox) (Math|Vector|MakeVector (Variables|Default|GetLength) 3e+02 75.0) true))