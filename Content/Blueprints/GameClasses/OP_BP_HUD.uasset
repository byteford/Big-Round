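; HUD class that creates the game's UMG screens: main menu, pause, win, lose, cutscene box, in-game HUD and achievement popups.
; Draw functions spawn each widget, most storing the calling player controller; pause and cutscene also switch to UI-only input.
; Achievements arriving while one is displayed are queued as prebuilt widgets, which Tick shows once the display flag is clear.
; DrawHUD renders a custom cursor texture at the mouse position.
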(event EventDrawHUD
  (params (SizeX :type Integer) (SizeY :type Integer))
  (bind _returnvalue (Game|GetPlayerController 0))
  (bind _returnvalue_2 (Math|Float|MakeLiteralFloat 0.0))
  (bind _cursersize (Variables|Default|GetCurserSize))
  (bind (_sizex _sizey) (HUD|GetViewportSize _returnvalue))
  (bind (_locationx _locationy) (Game|Player|GetMousePosition _returnvalue))
  (bind _returnvalue_3 (/ _returnvalue_2 2.0))
  (bind _returnvalue_4 (* _cursersize 0.5))
  (Class|HUD|DrawTextureSimple (Variables|Default|GetCursorTexture) (- (- (+ (/ (Math|Conversions|ToFloat(Integer) (- SizeX _sizex)) 2.0) _locationx) _returnvalue_3) _returnvalue_4) (- (- (+ (/ (Math|Conversions|ToFloat(Integer) (- SizeY _sizey)) 2.0) _locationy) _returnvalue_3) _returnvalue_4) 1.0 false))

(event EventTick
  (params (DeltaSeconds :type Float%20%28single-precision%29))
  (bind _achievementwidgetqueue (Variables|Default|GetAchievementWidgetQueue))
  (bind _item (Utilities|Array|Get(acopy) _achievementwidgetqueue))
  (if (!= (Utilities|Array|Length (Variables|Default|GetAchievementWidgetQueue)) 0)
    (if (not (Variables|Default|GetAchievementWidgetOnDisplay))
      (CallFunction|DrawAchievementHUDfromQueue _item)
      (Utilities|Array|RemoveItem _achievementwidgetqueue _item))))

(fn ConstructionScript)

(fn DrawMainMenuHUD
  (params (PC%20Ref :type OP%20BP%20Player%20Controller%20Object%20Reference))
  (bind _returnvalue (UserInterface|CreateWidget "/Game/Blueprints/UMG/OP_UMG_MainMenu.OP_UMG_MainMenu_C"))
  (UserInterface|Viewport|AddtoViewport _returnvalue 0)
  (Variables|/Game/Blueprints/UMG/OP_UMG_MainMenu.OP_UMG_MainMenu_C|SetWhoSpawnedMe _returnvalue PC%20Ref))

(fn DrawPauseMenuHUD
  (params (PC%20Ref :type OP%20BP%20Player%20Controller%20Object%20Reference))
  (bind _returnvalue (UserInterface|CreateWidget "/Game/Blueprints/UMG/OP_UMG_PauseMenu.OP_UMG_PauseMenu_C"))
  (UserInterface|Viewport|AddtoViewport _returnvalue 0)
  (Variables|/Game/Blueprints/UMG/OP_UMG_PauseMenu.OP_UMG_PauseMenu_C|SetWhoSpawnedMe _returnvalue PC%20Ref)
  (Input|SetInputModeUIOnly PC%20Ref _returnvalue false))

(fn DrawWinLevelHUD
  (params (PC%20Ref :type OP%20BP%20Player%20Controller%20Object%20Reference))
  (bind _returnvalue (UserInterface|CreateWidget "/Game/Blueprints/UMG/OP_UMG_WinLevel.OP_UMG_WinLevel_C"))
  (UserInterface|Viewport|AddtoViewport _returnvalue 0)
  (Variables|/Game/Blueprints/UMG/OP_UMG_WinLevel.OP_UMG_WinLevel_C|SetWhoSpawnedMe _returnvalue PC%20Ref))

(fn DrawinGameHUD
  (bind _returnvalue (UserInterface|CreateWidget "/Game/Blueprints/UMG/OP_UMG_InGameHUD.OP_UMG_InGameHUD_C"))
  (UserInterface|Viewport|AddtoViewport _returnvalue 0)
  (Variables|Default|SetInGameHUDRef _returnvalue))

(fn SetBonusRelicHUD
  (Appearance|SetBrushfromTexture (Variables|/Game/Blueprints/UMG/OP_UMG_InGameHUD.OP_UMG_InGameHUD_C|GetIMG_BonusRelic (Variables|Default|GetInGameHUDRef)) "/Game/Blueprints/UMG/HUDImages/OP_tx_hasrelic.OP_TX_hasrelic" true))

(fn DrawAchievementHUD
  (params (NewParam :type OP%20Struct%20Achievement%20Structure))
  (bind (_achievementname _achievementdescription _achievementtier) (Utilities|Struct|BreakOP_Struct_Achievement NewParam))
  (bind _returnvalue (UserInterface|CreateWidget "/Game/Blueprints/UMG/OP_UMG_Achievement.OP_UMG_Achievement_C"))
  (Variables|/Game/Blueprints/UMG/OP_UMG_Achievement.OP_UMG_Achievement_C|SetAchievement%20Name _returnvalue _achievementname)
  (Variables|/Game/Blueprints/UMG/OP_UMG_Achievement.OP_UMG_Achievement_C|SetAchievement%20Description _returnvalue _achievementdescription)
  (Variables|/Game/Blueprints/UMG/OP_UMG_Achievement.OP_UMG_Achievement_C|SetAchievementTier _returnvalue _achievementtier)
  (Variables|/Game/Blueprints/UMG/OP_UMG_Achievement.OP_UMG_Achievement_C|SetHUDRef _returnvalue self)
  (UserInterface|Viewport|AddtoViewport _returnvalue 0)
  (Variables|Default|SetAchievementWidgetOnDisplay true))

(fn CanDrawAchievementHUD
  (params (NewParam :type OP%20Struct%20Achievement%20Structure))
  (if (Variables|Default|GetAchievementWidgetOnDisplay)
    (CallFunction|DrawAchievementHUDtoQueue NewParam)
    (else
      (CallFunction|DrawAchievementHUD NewParam))))

(fn DrawAchievementHUDtoQueue
  (params (NewParam :type OP%20Struct%20Achievement%20Structure))
  (bind (_achievementname _achievementdescription _achievementtier) (Utilities|Struct|BreakOP_Struct_Achievement NewParam))
  (bind _returnvalue (UserInterface|CreateWidget "/Game/Blueprints/UMG/OP_UMG_Achievement.OP_UMG_Achievement_C"))
  (Variables|/Game/Blueprints/UMG/OP_UMG_Achievement.OP_UMG_Achievement_C|SetAchievement%20Name _returnvalue _achievementname)
  (Variables|/Game/Blueprints/UMG/OP_UMG_Achievement.OP_UMG_Achievement_C|SetAchievement%20Description _returnvalue _achievementdescription)
  (Variables|/Game/Blueprints/UMG/OP_UMG_Achievement.OP_UMG_Achievement_C|SetAchievementTier _returnvalue _achievementtier)
  (Variables|/Game/Blueprints/UMG/OP_UMG_Achievement.OP_UMG_Achievement_C|SetHUDRef _returnvalue self)
  (Utilities|Array|Add (Variables|Default|GetAchievementWidgetQueue) _returnvalue))

(fn DrawAchievementHUDfromQueue
  (params (NewParam :type OP%20UMG%20Achievement%20Object%20Reference))
  (UserInterface|Viewport|AddtoViewport NewParam 0)
  (Variables|Default|SetAchievementWidgetOnDisplay true))

(fn DrawLoseLevelHUD
  (params (PC%20Ref :type OP%20BP%20Player%20Controller%20Object%20Reference))
  (bind _returnvalue (UserInterface|CreateWidget "/Game/Blueprints/UMG/OP_UMG_Died.OP_UMG_Died_C"))
  (UserInterface|Viewport|AddtoViewport _returnvalue 0)
  (Variables|/Game/Blueprints/UMG/OP_UMG_Died.OP_UMG_Died_C|SetWhoSpawnedMe _returnvalue PC%20Ref))

(fn DrawCutsceneBoxHUD
  (params (PC%20Ref :type OP%20BP%20Player%20Controller%20Object%20Reference) (Text :type Text) (Fat :type Boolean))
  (bind _returnvalue (UserInterface|CreateWidget "/Game/Blueprints/UMG/OP_UMG_Cutscene.OP_UMG_Cutscene_C" 0 Text Fat))
  (UserInterface|Viewport|AddtoViewport _returnvalue 0)
  (Variables|/Game/Blueprints/UMG/OP_UMG_Cutscene.OP_UMG_Cutscene_C|SetWhoSpawnedMe _returnvalue PC%20Ref)
  (Input|SetInputModeUIOnly PC%20Ref _returnvalue false))