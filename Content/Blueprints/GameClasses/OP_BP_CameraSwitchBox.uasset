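; OP_BP_CameraSwitchBox is a placeable box trigger that switches the player character's camera while they are inside it.
; An actor overlap start calls CameraSwitchStart on OP_BP_Character, and the Box component's end overlap calls CameraSwitchEnd.
; Both events act only on that exact character class and leave the camera logic itself to the character.
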(event OnComponentEndOverlap(Box)
  (params (OtherActor :type Actor%20Object%20Reference) (OtherComp :type Primitive%20Component%20Object%20Reference) (OtherBodyIndex :type Integer))
  (if (== (Utilities|GetClass OtherActor) "/Game/Blueprints/OP_BP_Character.OP_BP_Character_C")
    (bind _asop_bp_character (Utilities|Casting|CastToOP_BP_Character OtherActor))
    (Default|CameraSwitchEnd _asop_bp_character)))

(event EventBeginPlay)

(event EventActorBeginOverlap
  (params (OtherActor :type Actor%20Object%20Reference))
  (if (== (Utilities|GetClass OtherActor) "/Game/Blueprints/OP_BP_Character.OP_BP_Character_C")
    (bind _asop_bp_character (Utilities|Casting|CastToOP_BP_Character OtherActor))
    (Default|CameraSwitchStart _asop_bp_character)))

(event EventTick
  (params (DeltaSeconds :type Float%20%28single-precision%29)))

(fn ConstructionScript)