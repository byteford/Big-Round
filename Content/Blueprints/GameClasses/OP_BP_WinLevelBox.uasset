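; OP_BP_WinLevelBox is a level-completion trigger that ends the level when the player character enters it carrying the relic.
; Each Tick it runs a box overlap query for OP_BP_Character pawns, sized by BoxSize, which the construction script also applies to the Box component.
; If the first character found has the relic, it disables that character's movement and calls its WinLevel once through a DoOnce.
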(event EventBeginPlay)

(event EventActorBeginOverlap
  (params (OtherActor :type Actor%20Object%20Reference))
  (if (== (Utilities|GetClass OtherActor) "/Game/Blueprints/OP_BP_Character.OP_BP_Character_C")
    _))

(event EventTick
  (params (DeltaSeconds :type Float%20%28single-precision%29))
  (bind _outactors (Class|KismetSystemLibrary|BoxOverlapActorsNEW (Transformation|GetWorldLocation (Variables|Default|GetBox)) (Variables|Default|GetBox%20Size) (Utilities|Array|MakeArray "ObjectTypeQuery3") "/Game/Blueprints/OP_BP_Character.OP_BP_Character_C"))
  (if (not (== (Utilities|Array|Length _outactors) 0))
    (bind _asop_bp_character (Utilities|Casting|CastToOP_BP_Character (Utilities|Array|Get(acopy) _outactors)))
    (if (Variables|/Game/Blueprints/OP_BP_Character.OP_BP_Character_C|GetHasRelic _asop_bp_character)
      (Variables|/Game/Blueprints/OP_BP_Character.OP_BP_Character_C|SetCanMove _asop_bp_character false)
      (Utilities|FlowControl|DoOnce false
        (:Completed
          (Default|WinLevel _asop_bp_character))))))

(fn ConstructionScript
  (Components|Box|SetBoxExtent (Variables|Default|GetBox) (Variables|Default|GetBox%20Size) true))