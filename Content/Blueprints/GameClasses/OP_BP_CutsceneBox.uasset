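; OP_BP_CutsceneBox is a one-shot trigger volume that starts a text cutscene when the player character walks into it.
; On first overlap with an OP_BP_Character, it disables movement, reads the player's size and controller, and passes them with its Text to OP_BP_HUD's DrawCutsceneBoxHUD.
; An AlreadyTriggered flag blocks repeats, and the construction script sizes the box from the BoxSize variable.
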(event EventBeginPlay)

(event EventActorBeginOverlap
  (params (OtherActor :type Actor%20Object%20Reference))
  (if (not (Variables|Default|GetAlreadyTriggered))
    (if (== (Utilities|GetClass OtherActor) "/Game/Blueprints/OP_BP_Character.OP_BP_Character_C")
      (bind _asop_bp_character (Utilities|Casting|CastToOP_BP_Character OtherActor))
      (Variables|/Game/Blueprints/OP_BP_Character.OP_BP_Character_C|SetCanMove _asop_bp_character false)
      (bind _fat_ (Default|GetPlayerSize _asop_bp_character))
      (bind _playercont (Default|GetPlayerController _asop_bp_character))
      (bind _asop_bp_hud (Utilities|Casting|CastToOP_BP_HUD (HUD|GetHUD _playercont)))
      (Default|DrawCutsceneBoxHUD _asop_bp_hud _playercont (Variables|Default|GetText) _fat_)
      (Variables|Default|SetAlreadyTriggered true))))

(event EventTick
  (params (DeltaSeconds :type Float%20%28single-precision%29)))

(fn ConstructionScript
  (Components|Box|SetBoxExtent (Variables|Default|GetBox) (Variables|Default|GetBox%20Size) true))